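; BP_MovePlane is an actor that patrols along a referenced spline when StartMove is called and IsOpen is set.
; A timeline's play rate is derived from spline length and Speed, so travel speed stays independent of path length.
; The start time is offset by the actor's index over a total count, staggering instances along the path.
; Each update sets world location and rotation from the spline distance.
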(event `StartMove`
  (bind _timeline (`self.Timeline`))
  (bind _spline (`/Game/BluePrints/BP_SplinePath.Spline` (`self.Spline to follow`)))
  ; Patrol
  (set `self.Time to Complete` (/ (`SplineComponent.GetSplineLength` (`/Game/BluePrints/BP_SplinePath.Spline` (`self.Spline to follow`))) (`self.Speed`)))
  (if (`self.IsOpen`)
    (`TimelineComponent.SetPlayRate` _timeline (/ 1.0 (`self.Time to Complete`)))
    (`TimelineComponent.SetNewTime` _timeline (/ (+ (`self.Num`) -1.0) (`self.TotalNum`)))
    (bind (_direction _move_track) (`Timeline|Timeline`)
      (:`Update`
        (bind _returnvalue (`KismetMathLibrary.Lerp` 0.0 (`SplineComponent.GetSplineLength` _spline) _move_track))
        (`self.K2_SetActorLocationAndRotation` (`SplineComponent.GetLocationAtDistanceAlongSpline` _spline _returnvalue "World") (`SplineComponent.GetRotationAtDistanceAlongSpline` _spline _returnvalue "World"))))))

(fn `UserConstructionScript`)