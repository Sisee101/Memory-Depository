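; Enemy that either patrols a spline or idles at its start point with a timeline-driven yaw sweep.
; Patrol walks to the spline actor, then a length-scaled timeline drives its transform along the path.
; Seeing a pawn turns the spotlight red and chases the player, fires a slash effect, then resumes after a cooldown.
; An overlap sphere shows a prompt when the player can attack; Interact then kills it with an explosion effect.
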(event `self.ReceiveBeginPlay`
  (bind _capsulecomponent (`self.CapsuleComponent`))
  ; BeginPlay
  (set `self.IdleLocation` (`SceneComponent.K2_GetComponentLocation` _capsulecomponent))
  (bind _output_get (set `self.IdleRotation` (`SceneComponent.K2_GetComponentRotation` _capsulecomponent)))
  (if (`self.CanPatrol?`)
    (set `self.Time to Complete` (/ (`SplineComponent.GetSplineLength` (`/Game/BluePrints/BP_SplinePath.Spline` (`self.Spline to follow`))) (`self.PatrolSpeed`)))
    (`self.Patrol`)
    (else
      (`self.Idle`))))

(event `Idle`
  ; Idle
  (if (not (`self.IsDead`))
    (`|AIMoveTo` self (`self.IdleLocation`) null 1.0
      (:`OnSuccess`
        (`SceneComponent.K2_SetWorldRotation` (`self.CapsuleComponent`) (stale `self.ReceiveBeginPlay` _output_get) false false)
        (bind (_direction _rotate) (`Timeline|TL_Rotate` :!via `PlayFromStart`)
          (:`Update`
            (`SceneComponent.K2_AddRelativeRotation` (`self.CapsuleComponent`) (`KismetMathLibrary.MakeRotator` 0.0 0.0 (* _rotate 1.0)) false false)))))))

(event `Patrol`
  (bind _returnvalue_location (`KismetMathLibrary.BreakTransform` (`self.GetTransform` (`self.Spline to follow`))))
  (bind _spline (`/Game/BluePrints/BP_SplinePath.Spline` (`self.Spline to follow`)))
  ; Patrol
  (if (not (`self.IsDead`))
    (`|AIMoveTo` self _returnvalue_location null 1.0
      (:`OnSuccess`
        (`TimelineComponent.SetPlayRate` (`self.TL_Patrol`) (/ 1.0 (`self.Time to Complete`)))
        (bind (_direction _move_track) (`Timeline|TL_Patrol` :!via `PlayFromStart`)
          (:`Update`
            (bind _returnvalue (`KismetMathLibrary.Lerp` 0.0 (`SplineComponent.GetSplineLength` _spline) _move_track))
            (`self.K2_SetActorLocationAndRotation` (`SplineComponent.GetLocationAtDistanceAlongSpline` _spline _returnvalue "World") (`SplineComponent.GetRotationAtDistanceAlongSpline` _spline _returnvalue "World"))))))))

(event `self.PawnSensing.OnSeePawn`
  (params (Pawn :type "Pawn Object Reference"))
  ; ChasePlayer
  (if (not (`self.IsDead`))
    (`self.Chase Player`)))

(event `Chase Player`
  (bind _returnvalue (`self.K2_GetActorRotation`))
  ; ChasePlayer
  (`LightComponent.SetLightColor` (`self.SpotLight`) (struct :`R` 1.0 :`G` 0.055493 :`A` 1.0) true)
  (`TimelineComponent.Stop` (`self.TL_Rotate`))
  (`TimelineComponent.Stop` (`self.TL_Patrol`))
  (`|AIMoveTo` self (0.0 0.0 0.0) (`GameplayStatics.GetPlayerCharacter` 0) 300.0
    (:`OnSuccess`
      (if (`self.Can Attack?`)
        (`NiagaraFunctionLibrary.SpawnSystemAtLocation` "/Game/MixedVFX/Particles/Slashes/SeparateParts/Hits/NS_FireSlash_Hit.NS_FireSlash_Hit" (+ (`self.K2_GetActorLocation`) (* (`KismetMathLibrary.GetForwardVector` _returnvalue) 300)) _returnvalue)
        (set `self.Can Attack?` false)
        (`KismetSystemLibrary.Delay` 4.0)
        (set `self.Can Attack?` true)
        (`LightComponent.SetLightColor` (`self.SpotLight`) (struct :`R` 0.243837 :`G` 0.884438 :`B` 1.0 :`A` 1.0) true)
        (if (`self.CanPatrol?`)
          (`self.Patrol`)
          (else
            (`self.Idle`)))))))

(event `/Game/BluePrints/BPI_Interact.Interact`
  ; Dead
  (bind _asbp_third_person_character (cast `/Game/ThirdPerson/Blueprints/BP_ThirdPersonCharacter` (`GameplayStatics.GetPlayerCharacter` 0)))
  (if (`/Game/ThirdPerson/Blueprints/BP_ThirdPersonCharacter.PlayerCanAttack?` _asbp_third_person_character)
    (`self.Dead`)))

(event `Dead`
  ; Dead
  (`TimelineComponent.Stop` (`self.TL_Patrol`))
  (`TimelineComponent.Stop` (`self.TL_Rotate`))
  (set `self.IsDead` true)
  (`NiagaraFunctionLibrary.SpawnSystemAtLocation` "/Game/MixedVFX/Particles/Explosions/NS_ExplosionMidAirSmall.NS_ExplosionMidAirSmall" (`self.K2_GetActorLocation`) (`self.K2_GetActorRotation`) (0.01 0.01 0.01))
  (`KismetSystemLibrary.Delay` 0.5)
  (`SceneComponent.SetVisibility` (`self.SpotLight`) false false))

(event `self.Sphere.OnComponentBeginOverlap`
  (params (OverlappedComponent :type "PrimitiveComponent Object Reference") (OtherActor :type "Actor Object Reference") (OtherComp :type "PrimitiveComponent Object Reference") (OtherBodyIndex :type Integer) (bFromSweep :type Boolean) (SweepResult :type "HitResult Structure (by ref)"))
  (bind _asbp_third_person_character (cast `/Game/ThirdPerson/Blueprints/BP_ThirdPersonCharacter` (`GameplayStatics.GetPlayerCharacter` 0)))
  (if (`/Game/ThirdPerson/Blueprints/BP_ThirdPersonCharacter.PlayerCanAttack?` _asbp_third_person_character)
    (`SceneComponent.SetVisibility` (`self.Widget`) true false)))

(event `self.Sphere.OnComponentEndOverlap`
  (params (OverlappedComponent :type "PrimitiveComponent Object Reference") (OtherActor :type "Actor Object Reference") (OtherComp :type "PrimitiveComponent Object Reference") (OtherBodyIndex :type Integer))
  (`SceneComponent.SetVisibility` (`self.Widget`) false false))

(fn `UserConstructionScript`)