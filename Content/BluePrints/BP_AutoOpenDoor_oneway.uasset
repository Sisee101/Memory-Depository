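; BP_AutoOpenDoor_oneway is a sliding door that opens automatically from one side only and has no closing logic.
; Overlapping Boxcollision plays a timeline that slides LeftDoor1 along local Y and sets Opened on update.
; Overlapping NotOpen before that shows a "cannot open from this side" widget (WBP_不能从这一侧打开) for two seconds.
; Neither trigger checks which actor overlaps it.
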(event `self.Boxcollision.OnComponentBeginOverlap`
  (params (OverlappedComponent :type "PrimitiveComponent Object Reference") (OtherActor :type "Actor Object Reference") (OtherComp :type "PrimitiveComponent Object Reference") (OtherBodyIndex :type Integer) (bFromSweep :type Boolean) (SweepResult :type "HitResult Structure (by ref)"))
  (bind (_direction _alpha) (`Timeline|TL_OpenDoor`)
    (:`Update`
      (`SceneComponent.K2_SetRelativeLocation` (`self.LeftDoor1`) (`KismetMathLibrary.MakeVector` 0.0 (`KismetMathLibrary.Lerp` 0.0 300.0 _alpha) -300.0) false false)
      (set `self.Opened` true))))

(event `self.not open.OnComponentBeginOverlap`
  (params (OverlappedComponent :type "PrimitiveComponent Object Reference") (OtherActor :type "Actor Object Reference") (OtherComp :type "PrimitiveComponent Object Reference") (OtherBodyIndex :type Integer) (bFromSweep :type Boolean) (SweepResult :type "HitResult Structure (by ref)"))
  (if (not (`self.Opened`))
    (bind _returnvalue (`|CreateWidget` "/Game/UI/WBP_不能从这一侧打开.WBP_不能从这一侧打开_C"))
    (`UserWidget.AddToViewport` _returnvalue 0)
    (`KismetSystemLibrary.Delay` 2.0)
    (`Widget.RemoveFromParent` _returnvalue)))

(fn `UserConstructionScript`)