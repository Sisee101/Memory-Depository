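; BP_Reading is an interactable note that opens a reading screen, WBP_电磁干扰留言 (electromagnetic interference message).
; A sphere trigger shows and hides the actor's Widget component on any overlap begin and end.
; Interact flags the player's BP_ThirdPersonCharacter as in interaction, adds the note widget to the viewport, shows the mouse cursor and pauses the game.
; Closing the note and undoing those states are not handled here.
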(event `self.Interact`
  (bind _asbp_third_person_character (cast `/Game/ThirdPerson/Blueprints/BP_ThirdPersonCharacter` (`GameplayStatics.GetPlayerCharacter` 0)))
  (set `/Game/ThirdPerson/Blueprints/BP_ThirdPersonCharacter.In Interaction?` true _asbp_third_person_character)
  (bind _returnvalue (`|CreateWidget` "/Game/UI/WBP_电磁干扰留言.WBP_电磁干扰留言_C"))
  (`UserWidget.AddToViewport` _returnvalue 0)
  (set `PlayerController.bShowMouseCursor` true (`GameplayStatics.GetPlayerController` 0))
  (`GameplayStatics.SetGamePaused` true)
  (`KismetSystemLibrary.PrintString` "note"))

(event `self.Sphere.OnComponentBeginOverlap`
  (params (OverlappedComponent :type "PrimitiveComponent Object Reference") (OtherActor :type "Actor Object Reference") (OtherComp :type "PrimitiveComponent Object Reference") (OtherBodyIndex :type Integer) (bFromSweep :type Boolean) (SweepResult :type "HitResult Structure (by ref)"))
  (`SceneComponent.SetVisibility` (`self.Widget`) true false))

(event `self.Sphere.OnComponentEndOverlap`
  (params (OverlappedComponent :type "PrimitiveComponent Object Reference") (OtherActor :type "Actor Object Reference") (OtherComp :type "PrimitiveComponent Object Reference") (OtherBodyIndex :type Integer))
  (`SceneComponent.SetVisibility` (`self.Widget`) false false))

(fn `UserConstructionScript`)