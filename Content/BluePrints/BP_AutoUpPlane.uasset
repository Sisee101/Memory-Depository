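; BP_AutoUpPlane is an actor that automatically moves its LeftDoor1 component vertically, apparently as a rising platform, when something overlaps its Box.
; After a short delay, it plays the TL_OpenDoor timeline, interpolating the component's relative Z by Height from a hardcoded base offset.
; Play rate derives from MoveSpeed over Height, so speed stays independent of travel distance.
; The overlap is unfiltered, and no return movement exists.
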(event `self.Box.OnComponentBeginOverlap`
  (params (OverlappedComponent :type "PrimitiveComponent Object Reference") (OtherActor :type "Actor Object Reference") (OtherComp :type "PrimitiveComponent Object Reference") (OtherBodyIndex :type Integer) (bFromSweep :type Boolean) (SweepResult :type "HitResult Structure (by ref)"))
  (`KismetSystemLibrary.Delay` 1.5)
  (`TimelineComponent.SetPlayRate` (`self.TL_OpenDoor`) (`KismetMathLibrary.Abs` (/ 1.0 (/ (`self.Height`) (`self.MoveSpeed`)))))
  (bind (_direction _alpha) (`Timeline|TL_OpenDoor`)
    (:`Update`
      (`SceneComponent.K2_SetRelativeLocation` (`self.LeftDoor1`) (`KismetMathLibrary.MakeVector` 500.0 -155.0 (+ (`KismetMathLibrary.Lerp` 0.0 (`self.Height`) _alpha) -300.0)) false false))))

(fn `UserConstructionScript`)