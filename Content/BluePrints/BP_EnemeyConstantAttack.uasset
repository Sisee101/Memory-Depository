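; Stationary enemy that rotates on a timeline while idle and fires a repeatable forward attack when it sees a pawn.
; Pawn sensing stops the rotation, reddens the spotlight, plays a sound and, after a short gated delay, spawns a slash effect, with no damage applied here.
; A sphere overlap shows a widget when the player can attack; interacting then disables the enemy.
; The explosion and light-off death effects are unconnected.
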(event `self.ReceiveBeginPlay`
  (bind _capsulecomponent (`self.CapsuleComponent`))
  ; BeginPlay
  (set `self.IdleLocation` (`SceneComponent.K2_GetComponentLocation` _capsulecomponent))
  (bind _output_get (set `self.IdleRotation` (`SceneComponent.K2_GetComponentRotation` _capsulecomponent)))
  (`self.Idle`))

(event `Idle`
  ; Idle
  (if (not (`self.IsDead`))
    (`SceneComponent.K2_SetWorldRotation` (`self.CapsuleComponent`) (stale `self.ReceiveBeginPlay` _output_get) false false)
    (bind (_direction _rotate) (`Timeline|TL_Rotate` :!via `PlayFromStart`)
      (:`Update`
        (`SceneComponent.K2_AddRelativeRotation` (`self.CapsuleComponent`) (`KismetMathLibrary.MakeRotator` 0.0 0.0 (* _rotate 1.0)) false false)))))

(event `self.PawnSensing.OnSeePawn`
  (params (Pawn :type "Pawn Object Reference"))
  ; ChasePlayer
  (if (not (`self.IsDead`))
    (`self.Chase Player`)))

(event `Chase Player`
  (bind _returnvalue (`self.K2_GetActorRotation`))
  ; ChasePlayer
  (`LightComponent.SetLightColor` (`self.SpotLight`) (struct :`R` 1.0 :`G` 0.055493 :`A` 1.0) true)
  (`TimelineComponent.Stop` (`self.TL_Rotate`))
  (if (`self.canattack`)
    (`GameplayStatics.PlaySoundAtLocation` "/Game/Audio/zapsplat_science_fiction_weapon_large_cannon_rpg_launcher_fire_blast_beeps_robotic_004_89854.zapsplat_science_fiction_weapon_large_cannon_rpg_launcher_fire_blast_beeps_robotic_004_89854" (0.0 0.0 0.0) (struct) 1.0 1.0 0.0 null null null null)
    (set `self.canattack` false)
    (`KismetSystemLibrary.Delay` 0.8)
    (`NiagaraFunctionLibrary.SpawnSystemAtLocation` "/Game/MixedVFX/Particles/Slashes/SeparateParts/Hits/NS_FireSlash_Hit.NS_FireSlash_Hit" (+ (`self.K2_GetActorLocation`) (* (`KismetMathLibrary.GetForwardVector` _returnvalue) 400)) _returnvalue)
    (set `self.canattack` true)))

(event `self.Interact`
  ; Dead
  (bind _asbp_third_person_character (cast `/Game/ThirdPerson/Blueprints/BP_ThirdPersonCharacter` (`GameplayStatics.GetPlayerCharacter` 0)))
  (if (`/Game/ThirdPerson/Blueprints/BP_ThirdPersonCharacter.PlayerCanAttack?` _asbp_third_person_character)
    (`self.Dead`)))

(event `Dead`
  ; Dead
  (`TimelineComponent.Stop` (`self.TL_Rotate`))
  (set `self.IsDead` true))

(event `self.Sphere.OnComponentBeginOverlap`
  (params (OverlappedComponent :type "PrimitiveComponent Object Reference") (OtherActor :type "Actor Object Reference") (OtherComp :type "PrimitiveComponent Object Reference") (OtherBodyIndex :type Integer) (bFromSweep :type Boolean) (SweepResult :type "HitResult Structure (by ref)"))
  (bind _asbp_third_person_character (cast `/Game/ThirdPerson/Blueprints/BP_ThirdPersonCharacter` OtherActor))
  (if (`/Game/ThirdPerson/Blueprints/BP_ThirdPersonCharacter.PlayerCanAttack?` _asbp_third_person_character)
    (`SceneComponent.SetVisibility` (`self.Widget`) true false)))

(event `self.Sphere.OnComponentEndOverlap`
  (params (OverlappedComponent :type "PrimitiveComponent Object Reference") (OtherActor :type "Actor Object Reference") (OtherComp :type "PrimitiveComponent Object Reference") (OtherBodyIndex :type Integer))
  (`SceneComponent.SetVisibility` (`self.Widget`) false false))

(fn `UserConstructionScript`)