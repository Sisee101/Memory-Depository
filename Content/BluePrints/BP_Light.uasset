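; BP_Light is a light Blueprint that plays a timed power-on sequence when its PowerOn event is called.
; PowerOn plays the MS_poweron sound at a hardcoded world location, then uses chained delays to switch four sphere components and a Cloud component, one by one, to the MI_Unlit_Mask material.
; The sequence ends by hiding the SpotLight, with no logic to reverse it.
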(event `Power On`
  (`GameplayStatics.PlaySoundAtLocation` "/Game/Audio/MS_poweron.MS_poweron" (-2692.851695 -1366.451669 628.024611) (struct) 1.0 1.0 0.0 null null null null)
  (`KismetSystemLibrary.Delay` 2.8)
  (`PrimitiveComponent.SetMaterial` (`self.Sphere3`) 0 "/InterchangeAssets/gltf/MaterialInstances/MI_Unlit_Mask.MI_Unlit_Mask")
  (`KismetSystemLibrary.Delay` 0.4)
  (`PrimitiveComponent.SetMaterial` (`self.Sphere1`) 0 "/InterchangeAssets/gltf/MaterialInstances/MI_Unlit_Mask.MI_Unlit_Mask")
  (`KismetSystemLibrary.Delay` 0.4)
  (`PrimitiveComponent.SetMaterial` (`self.Sphere`) 0 "/InterchangeAssets/gltf/MaterialInstances/MI_Unlit_Mask.MI_Unlit_Mask")
  (`KismetSystemLibrary.Delay` 1.5)
  (`PrimitiveComponent.SetMaterial` (`self.Sphere2`) 0 "/InterchangeAssets/gltf/MaterialInstances/MI_Unlit_Mask.MI_Unlit_Mask")
  (`KismetSystemLibrary.Delay` 0.5)
  (`PrimitiveComponent.SetMaterial` (`self.cloud`) 0 "/InterchangeAssets/gltf/MaterialInstances/MI_Unlit_Mask.MI_Unlit_Mask")
  (`SceneComponent.SetVisibility` (`self.SpotLight`) false false))

(fn `UserConstructionScript`)