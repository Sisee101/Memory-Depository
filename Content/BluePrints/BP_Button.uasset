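; BP_Button is an interactable button that triggers either a door or a conveyor (Chuansongdai), chosen by TargetType.
; Door mode opens the TargetActor BP_BottonOpenDoor, requiring the player's HaveKey when IsLocked.
; Conveyor mode requires the player's HavePowerOn, then starts every BP_MovePlane in the level, ignoring TargetActor.
; Failed checks show a WBP_需要钥匙 tip widget, which only the door branch removes after a delay.
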(event `/Game/BluePrints/BPI_Interact.Interact`
  (switch `/Game/BluePrints/E_ButtonInteractType` (`self.TargetType`)
    (:`NewEnumerator0`
      (if (`self.IsLocked?`)
        (bind _asbp_third_person_character (cast `/Game/ThirdPerson/Blueprints/BP_ThirdPersonCharacter` (`GameplayStatics.GetPlayerCharacter` 0)))
        (if (`/Game/ThirdPerson/Blueprints/BP_ThirdPersonCharacter.HaveKey?` _asbp_third_person_character)
          (bind _asbp_botton_open_door (cast `/Game/BluePrints/BP_BottonOpenDoor` (`self.TargetActor`)))
          (`/Game/BluePrints/BP_BottonOpenDoor.OpenDoor` _asbp_botton_open_door)
          (else
            (bind _returnvalue (`|CreateWidget` "/Game/UI/WBP_需要钥匙.WBP_需要钥匙_C"))
            (`TextBlock.SetText` (`/Game/UI/WBP_需要钥匙.tiptiptext` _returnvalue) (`KismetTextLibrary.Conv_StringToText` (`self.tiptext`)))
            (`UserWidget.AddToViewport` _returnvalue 0)
            (`KismetSystemLibrary.Delay` 2.0)
            (`Widget.RemoveFromParent` _returnvalue)))
        (else
          (bind _asbp_botton_open_door_2 (cast `/Game/BluePrints/BP_BottonOpenDoor` (`self.TargetActor`)))
          (`/Game/BluePrints/BP_BottonOpenDoor.OpenDoor` _asbp_botton_open_door_2))))
    (:`NewEnumerator2`
      (bind _asbp_third_person_character_2 (cast `/Game/ThirdPerson/Blueprints/BP_ThirdPersonCharacter` (`GameplayStatics.GetPlayerCharacter` 0)))
      (if (`/Game/ThirdPerson/Blueprints/BP_ThirdPersonCharacter.HavePowerOn?` _asbp_third_person_character_2)
        (bind _outactors (`GameplayStatics.GetAllActorsOfClass` "/Game/BluePrints/BP_MovePlane.BP_MovePlane_C"))
        (for _array_element _outactors
          (`/Game/BluePrints/BP_MovePlane.StartMove` _array_element))
        (else
          (bind _returnvalue_2 (`|CreateWidget` "/Game/UI/WBP_需要钥匙.WBP_需要钥匙_C"))
          (`TextBlock.SetText` (`/Game/UI/WBP_需要钥匙.tiptiptext` _returnvalue_2) "需要启动电力")
          (`UserWidget.AddToViewport` _returnvalue_2 0)
          (`KismetSystemLibrary.Delay` 2.0))))))

(fn `UserConstructionScript`)